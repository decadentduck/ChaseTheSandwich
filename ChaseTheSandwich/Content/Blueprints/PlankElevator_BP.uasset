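; PlankElevator_BP is an elevator that rises by a set Height when the player enters its Box trigger and returns after the player leaves.
; BeginPlay caches the player pawn and both endpoints, and two separate timelines lerp the root between them.
; Overlap plays the rising timeline; end overlap waits briefly, then plays the other in reverse.
; HaveUsed blocks retriggering once raised and clears when the descent finishes.
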(event OnComponentBeginOverlap(Box)
  (params (OverlappedComponent :type Primitive%20Component%20Object%20Reference) (OtherActor :type Actor%20Object%20Reference) (OtherComp :type Primitive%20Component%20Object%20Reference) (OtherBodyIndex :type Integer) (bFromSweep :type Boolean) (SweepResult :type Hit%20Result%20Structure%20%28by%20ref%29))
  (if (== OtherActor (Variables|Default|Getplayer))
    (if (not (Variables|Default|GetHaveUsed?))
      (bind _newtrack_1 (Timeline|Elevator_Rising PlayFromStart)
        (:Update
          (Transformation|SetRelativeLocation (Variables|Default|GetDefaultSceneRoot) (Math|Vector|Lerp(Vector) (Variables|Default|GetStartPoint) (Variables|Default|GetEndPoint) _newtrack_1) false false))
        (:Finished
          (Variables|Default|SetHaveUsed? true))))))

(event OnComponentEndOverlap(Box)
  (params (OverlappedComponent :type Primitive%20Component%20Object%20Reference) (OtherActor :type Actor%20Object%20Reference) (OtherComp :type Primitive%20Component%20Object%20Reference) (OtherBodyIndex :type Integer))
  (if (== OtherActor (Variables|Default|Getplayer))
    (Utilities|FlowControl|Delay 0.2)
    (bind _newtrack_1 (Timeline|Timeline_0 ReverseFromEnd)
      (:Update
        (Transformation|SetRelativeLocation (Variables|Default|GetDefaultSceneRoot) (Math|Vector|Lerp(Vector) (Variables|Default|GetStartPoint) (Variables|Default|GetEndPoint) _newtrack_1) false false))
      (:Finished
        (Variables|Default|SetHaveUsed? false)))))

(event EventBeginPlay
  (Variables|Default|Setplayer (Game|Player|GetPlayerPawn 0))
  (bind _output_get (Variables|Default|SetStartPoint (Variables|/Script/Engine.SceneComponent|GetRelativeLocation (Variables|Default|GetDefaultSceneRoot))))
  (Variables|Default|SetEndPoint (+ _output_get (Math|Vector|MakeVector 0.0 0.0 (Variables|Default|Getheight)))))

(event Collision|EventActorBeginOverlap
  (params (OtherActor :type Actor%20Object%20Reference)))

(event EventTick
  (params (DeltaSeconds :type Float%20%28single-precision%29)))

(fn ConstructionScript)